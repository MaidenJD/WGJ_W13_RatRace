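; Base vehicle actor that drives along its spline once per Simulate call, apparently as one move in a turn-based game.
; A timeline moves and rotates the Vehicle component along the spline in local space, with a yaw correction of -90 degrees.
; On finish, it resets the component and offsets the actor by the spline's end location, ready for the next turn.
; The construction script gives the vehicle a random dark colour through a dynamic material instance.
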(event `Simulate`
  (bind (_returnvalue_x _returnvalue_y _returnvalue_z) (`KismetMathLibrary.BreakVector` (`SplineComponent.GetLocationAtTime` (`self.Spline`) 1.0 "Local" false)))
  (bind (_direction _time) (`Timeline|Timeline_0` :!via `PlayFromStart`)
    (:`Update`
      (bind (_returnvalue_x_2 _returnvalue_y_2 _returnvalue_z_2) (`KismetMathLibrary.BreakVector` (`SplineComponent.GetLocationAtTime` (`self.Spline`) _time "Local" false)))
      ;[1 1 1] Update Movement
      (`SceneComponent.K2_SetRelativeLocation` (`self.Vehicle`) (`KismetMathLibrary.MakeVector` _returnvalue_x_2 _returnvalue_y_2 _returnvalue_z_2) false false)
      (bind (_returnvalue_roll _returnvalue_pitch _returnvalue_yaw) (`KismetMathLibrary.BreakRotator` (`SplineComponent.GetRotationAtTime` (`self.Spline`) _time "Local" false)))
      (`SceneComponent.K2_SetRelativeRotation` (`self.Vehicle`) (`KismetMathLibrary.MakeRotator` _returnvalue_roll _returnvalue_pitch (- _returnvalue_yaw 90.0)) false false))
    (:`Finished`
      ;[1 1 1] Reset Ready for next Turn
      (`SceneComponent.K2_SetRelativeLocationAndRotation` (`self.Vehicle`) (0.0 0.0 0.0) (struct :`Yaw` -90.0) false false)
      (`self.K2_AddActorLocalOffset` (`KismetMathLibrary.MakeVector` _returnvalue_x _returnvalue_y _returnvalue_z)))))

(fn `GenerateRandomColour`
  (params (ElementIndex :type Integer))
  (bind _returnvalue (`PrimitiveComponent.CreateDynamicMaterialInstance` (`self.Vehicle`) ElementIndex "/Game/Assets/Materials/Vehicles/MAT_Primary.MAT_Primary"))
  (`MaterialInstanceDynamic.SetVectorParameterValue` _returnvalue "Colour" (make `LinearColor` (`KismetMathLibrary.RandomFloatInRange` 0.0 0.5) (`KismetMathLibrary.RandomFloatInRange` 0.0 0.5) (`KismetMathLibrary.RandomFloatInRange` 0.25 0.5) 1.0)))

(fn `RandomiseColours`
  (`self.GenerateRandomColour` 0))

(fn `UserConstructionScript`
  (`self.RandomiseColours`))