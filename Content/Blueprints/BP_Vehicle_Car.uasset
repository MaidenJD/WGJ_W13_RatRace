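; Vehicle Blueprint for a car that repeatedly drives along its own spline, advancing the actor one path length per cycle.
; Tick samples the spline from the fractional part of game time over a two-second cycle and sets the Vehicle component's relative location and rotation, with a yaw correction.
; Near each cycle's end, a DoOnce resets the component and offsets the actor by the spline's endpoint, leaving actor rotation unchanged.
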(event `self.ReceiveTick`
  (params (DeltaSeconds :type "Float (single-precision)"))
  (bind (_returnvalue_x _returnvalue_y _returnvalue_z) (`KismetMathLibrary.BreakVector` (`SplineComponent.GetLocationAtTime` (`self.Spline`) 1.0 "Local" false)))
  (bind _returnvalue (`KismetMathLibrary.Fraction` (/ (`GameplayStatics.GetTimeSeconds`) 2.0)))
  (bind (_returnvalue_x_2 _returnvalue_y_2 _returnvalue_z_2) (`KismetMathLibrary.BreakVector` (`SplineComponent.GetLocationAtTime` (`self.Spline`) _returnvalue "Local" false)))
  (bind (_returnvalue_roll _returnvalue_pitch _returnvalue_yaw) (`KismetMathLibrary.BreakRotator` (`SplineComponent.GetRotationAtTime` (`self.Spline`) _returnvalue "Local" false)))
  ;[1 1 1] Update Movement
  (`SceneComponent.K2_SetRelativeLocation` (`self.Vehicle`) (`KismetMathLibrary.MakeVector` _returnvalue_x_2 _returnvalue_y_2 _returnvalue_z_2) false false)
  (`SceneComponent.K2_SetRelativeRotation` (`self.Vehicle`) (`KismetMathLibrary.MakeRotator` _returnvalue_roll _returnvalue_pitch (- _returnvalue_yaw 90.0)) false false)
  (if (>= _returnvalue 0.9925)
    (`/Engine/EditorBlueprintResources/StandardMacros.DoOnce` false :!label _label
      (:`Completed`
        ;[1 1 1] Reset Ready for next Turn
        (`SceneComponent.K2_SetRelativeLocationAndRotation` :`self` (`self.Vehicle`) :`NewLocation` (0.0 0.0 80.0))
        (`self.K2_AddActorLocalOffset` (`KismetMathLibrary.MakeVector` _returnvalue_x _returnvalue_y _returnvalue_z))))
    (else
      (goto _label :!via `Reset`))))

(fn `UserConstructionScript`)