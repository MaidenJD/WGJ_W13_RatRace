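; Main game mode for a turn-based traffic puzzle that builds the level and runs the vehicle simulation.
; BeginPlay spawns vehicles from the GameInstance's puzzle data on a lane-and-slot grid, centring longer vehicles across their slots and placing bikes between lanes.
; Each turn orders vehicles front to back using stepped cross-lane line traces, then simulates them one by one through a delayed recursive event.
; Ending a turn increments the counter and restarts the simulation.
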(event `self.ReceiveBeginPlay`
  (`self.SetupEventBindings`)
  (bind _output_get (set `self.RefGI` (cast `/Game/Blueprints/Core/GI_Main` (`GameplayStatics.GetGameInstance`) :!pure true)))
  (bind _puzzletoload (`/Game/Blueprints/Core/GI_Main.PuzzleToLoad` _output_get))
  (bind _lanedata (`Puzzle.GetLaneData` _puzzletoload))
  ;[1 1 1] Working out largest lane length
  (for _array_element (break `LaneData` (`BlueprintMapLibrary.Map_Find` _lanedata 1))
    (set `self.SlotTotal` (+ (`self.SlotTotal`) (select `EVehicleType` _array_element :`VT_None` 1 :`VT_Car` 1 :`VT_Truck` 2 :`VT_Bus` 3))))
  ;[1 1 1] Saving Lane Count
  (bind _keys (`BlueprintMapLibrary.Map_Keys` _lanedata))
  (set `self.LaneTotal` (`|GetArrayItem` _keys (`KismetArrayLibrary.Array_LastIndex` _keys)))
  ;[1 1 1] Spawning Non-Bikes
  (for (_array_element_2 _array_index) _keys
    (set `self.WorkingSlotIndex` (`self.SlotTotal`))
    (for _array_element_3 (break `LaneData` (`BlueprintMapLibrary.Map_Find` _lanedata _array_element_2))
      (if (`|EnumInequality` _array_element_3 "VT_None")
        (bind _returnvalue (`|SpawnActorFromClass` (select `EVehicleType` _array_element_3 :`VT_Car` "/Game/Blueprints/Vehicles/BP_Vehicle_Car.BP_Vehicle_Car_C" :`VT_Truck` "/Game/Blueprints/Vehicles/BP_Vehicle_Truck.BP_Vehicle_Truck_C" :`VT_Bus` "/Game/Blueprints/Vehicles/BP_Vehicle_Bus.BP_Vehicle_Bus_C" :!type "Actor Class Reference") (`KismetMathLibrary.MakeTransform` (`KismetMathLibrary.MakeVector` (* (- 1.0 (select `EVehicleType` _array_element_3 :`VT_Car` (`KismetMathLibrary.Conv_IntToDouble` (`self.WorkingSlotIndex`)) :`VT_Truck` (/ (`KismetMathLibrary.Conv_IntToDouble` (+ (`self.WorkingSlotIndex`) (- (`self.WorkingSlotIndex`) 1))) 2.0) :`VT_Bus` (/ (`KismetMathLibrary.Conv_IntToDouble` (+ (`self.WorkingSlotIndex`) (- (`self.WorkingSlotIndex`) 2))) 2.0))) 500.0) (`KismetMathLibrary.Conv_IntToDouble` (* _array_index 420)))) "Undefined" "OverrideRootScale" null null))
        (bind _asbp_vehicle_base (cast `/Game/Blueprints/Vehicles/BP_Vehicle_Base` _returnvalue :!pure true))
        (`/Game/Blueprints/Vehicles/BP_Vehicle_Base.InitialiseVehicle` _asbp_vehicle_base self _array_element_2)
        (`KismetArrayLibrary.Array_Add` (`self.VehiclesInPuzzle`) _asbp_vehicle_base))
      (set `self.WorkingSlotIndex` (- (`self.WorkingSlotIndex`) (select `EVehicleType` _array_element_3 :`VT_None` 1 :`VT_Car` 1 :`VT_Truck` 2 :`VT_Bus` 3)))))
  (bind _bikedata (`Puzzle.GetBikeData` _puzzletoload))
  ;[1 1 1] Spawning Bikes
  (bind _keys_2 (`BlueprintMapLibrary.Map_Keys` _bikedata))
  (for (_array_element_4 _array_index_2) _keys_2
    (for _array_element_5 (break `BikeData` (`BlueprintMapLibrary.Map_Find` _bikedata _array_element_4))
      (bind _returnvalue_2 (`|SpawnActorFromClass` "/Game/Blueprints/Vehicles/BP_Vehicle_Bike.BP_Vehicle_Bike_C" (`KismetMathLibrary.MakeTransform` (`KismetMathLibrary.MakeVector` (`KismetMathLibrary.Conv_IntToDouble` (* (- 1 _array_element_5) 500)) (`KismetMathLibrary.Conv_IntToDouble` (+ (* _array_index_2 420) 210)))) "Undefined" "OverrideRootScale" null null))
      (`/Game/Blueprints/Vehicles/BP_Vehicle_Base.InitialiseVehicle` _returnvalue_2 self _array_element_4)
      (`KismetArrayLibrary.Array_Add` (`self.VehiclesInPuzzle`) _returnvalue_2))))

(event `SetupEventBindings`
  ;[1 1 1] Bind Sim Events
  (add `self.StartSimulation` (delegate `SimulationStarted`))
  (add `self.EndSimulation` (delegate `SimulationEnded`)))

(event `SimulationStarted`
  ;[1 1 1] Start Sim Loop
  (bind _simulationorder (`self.CalculateSimulationOrder`))
  (set `self.SimOrder` _simulationorder)
  (`self.SimulateNext` 0))

(event `SimulateNext`
  (params (SimIndex :type Integer))
  (bind _returnvalue (+ SimIndex 1))
  (bind _simulationstepdelay (`self.SimulationStepDelay`))
  ;[1 1 1] Simulate each vehicle with a delay between
  (`/Game/Blueprints/Vehicles/BP_Vehicle_Base.Simulate` (`|GetArrayItem` (`self.SimOrder`) SimIndex))
  (`KismetSystemLibrary.Delay` (/ (`self.SimulationStepDelay`) (`self.SimulationSpeedMultipler`)))
  (if (> _returnvalue (`KismetArrayLibrary.Array_LastIndex` (`self.SimOrder`)))
    (`KismetSystemLibrary.Delay` (/ (- (`KismetMathLibrary.Fraction` _simulationstepdelay) _simulationstepdelay) (`self.SimulationSpeedMultipler`)))
    (`self.EndSimulation`)
    (else
      (`self.SimulateNext` _returnvalue))))

(event `SimulationEnded`
  ;[1 1 1] Advance turn counter
  (`/Engine/EditorBlueprintResources/StandardMacros.IncrementInt` (`self.TurnCount`)
    (:`  `
      (`self.StartSimulation`))))

(fn `CalculateRayXPoints`
  (returns (FurthestCarX :type "Float (double-precision)") (ClosestCarX :type "Float (double-precision)"))
  (locals (closestCar :type "Float (double-precision)" :default 10000000000.0) (furthestCar :type "Float (double-precision)" :default -9999999827968.0) (numSlots :type Integer) (offsetSlots :type Integer) (slotsFromOrigin :type Integer))
  (bind _furthestcar (`local.furthestCar`))
  (bind _closestcar (`local.closestCar`))
  ;[1 1 1] Calculate Furthest and Closest Car
  (for _array_element (`self.VehiclesInPuzzle`)
    (bind _returnvalue_x (`KismetMathLibrary.BreakVector` (`self.K2_GetActorLocation` _array_element)))
    (`|VariableSetRef` (select `bool` (< _returnvalue_x _closestcar) :`false` (select `bool` (> _returnvalue_x _furthestcar) :`true` _furthestcar) :`true` _closestcar) _returnvalue_x))
  (return (`local.furthestCar`) (`local.closestCar`)))

(fn `CalculateSimulationOrder`
  (returns (SimulationOrder :type "Array of /Game/Blueprints/Vehicles/BP_Vehicle_Base Object Reference"))
  (locals (return :type "Array of /Game/Blueprints/Vehicles/BP_Vehicle_Base Object Reference") (Xpositions :type "Vector2D Structure"))
  (bind (_furthestcarx _closestcarx) (`self.CalculateRayXPoints`))
  (bind (_xpositions_x _xpositions_y) (`KismetMathLibrary.BreakVector2D` (`local.Xpositions`)))
  (bind _xpositions_x_2 (`KismetMathLibrary.BreakVector2D` (`local.Xpositions`)))
  (bind _output_get (set `local.Xpositions` (`KismetMathLibrary.MakeVector2D` _furthestcarx _closestcarx)))
  ;[1 1 1] Calculate Move Order
  (while (>= (`KismetMathLibrary.BreakVector2D` _output_get) (`.Y` (`KismetMathLibrary.BreakVector2D` _output_get)))
    (bind _outhits (`KismetSystemLibrary.LineTraceMulti` (`KismetMathLibrary.MakeVector` _xpositions_x_2 -420.0 150.0) (`KismetMathLibrary.MakeVector` _xpositions_x_2 (* (`self.LaneTotal`) 420.0) 150.0) "TraceTypeQuery1"))
    (for _array_element _outhits
      (bind _asbp_vehicle_base (cast `/Game/Blueprints/Vehicles/BP_Vehicle_Base` (`.HitActor` (`GameplayStatics.BreakHitResult` _array_element))))
      (`KismetArrayLibrary.Array_AddUnique` (`local.return`) _asbp_vehicle_base))
    (set `local.Xpositions` (`KismetMathLibrary.MakeVector2D` (- _xpositions_x 500.0) _xpositions_y)))
  (return (`local.return`)))

(fn `UserConstructionScript`)