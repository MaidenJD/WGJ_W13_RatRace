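; Vehicle base Blueprint that moves its Vehicle component along a Spline.
; Each Tick samples the spline at constant velocity, using game time clamped to two seconds, so motion runs once from world start rather than looping.
; It follows only X, Y and yaw, keeping the current height and offsetting yaw by -90 degrees.
; A fractional-time calculation is left unconnected.
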(event `self.ReceiveTick`
  (params (DeltaSeconds :type "Float (single-precision)"))
  (bind _spline (`self.Spline`))
  (bind _vehicle (`self.Vehicle`))
  (bind _returnvalue (`KismetMathLibrary.FClamp` (`GameplayStatics.GetTimeSeconds`) 0.0 2.0))
  (bind (_returnvalue_x _returnvalue_y _returnvalue_z) (`KismetMathLibrary.BreakVector` (`SceneComponent.K2_GetComponentLocation` _vehicle)))
  (bind (_returnvalue_x_2 _returnvalue_y_2) (`KismetMathLibrary.BreakVector` (`SplineComponent.GetLocationAtTime` _spline _returnvalue "World" true)))
  (bind (_returnvalue_roll _returnvalue_pitch _returnvalue_yaw) (`KismetMathLibrary.BreakRotator` (`SplineComponent.GetRotationAtTime` _spline _returnvalue "World" true)))
  (`SceneComponent.K2_SetWorldLocation` _vehicle (`KismetMathLibrary.MakeVector` _returnvalue_x_2 _returnvalue_y_2 _returnvalue_z) false false)
  (`SceneComponent.K2_SetWorldRotation` _vehicle (`KismetMathLibrary.MakeRotator` 0.0 0.0 (- _returnvalue_yaw 90.0)) false false))

(fn `UserConstructionScript`)